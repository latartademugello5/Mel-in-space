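; BP_MIS_CubeActor is an interactable cube that enlarges when the first-person player interacts with it.
; On BeginPlay it caches the player's BP_MIS_FirstPersonCharacter.
; Every Tick it polls that character's HitActor and DidInteract, setting its scale to a fixed enlarged size when it is the hit actor and interaction is flagged.
; Nothing restores the scale, and the Highlight Object section holds only a disabled overlap event.
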(event EventBeginPlay
  ;[0.15 0.15 0.15 0.5] Scale Functionality
  (bind _asbp_mis_first_person_character (Utilities|Casting|CastToBP_MIS_FirstPersonCharacter (Game|GetPlayerCharacter 0)))
  (Variables|Default|SetrefCharacter _asbp_mis_first_person_character))

(event Collision|EventActorBeginOverlap
  (params (OtherActor :type Actor%20Object%20Reference))
  ;[0.15 0.15 0.15 0.5] Highlight Object
)

(event EventTick
  (params (DeltaSeconds :type Float%20%28single-precision%29))
  (bind _refcharacter (Variables|Default|GetrefCharacter))
  ;[0.15 0.15 0.15 0.5] Scale Functionality
  (if (and (== self (Variables|/Game/Mel_In_Space_Additions/Blueprints/BP_MIS_FirstPersonCharacter.BP_MIS_FirstPersonCharacter_C|GetHit%20Actor _refcharacter)) (Variables|/Game/Mel_In_Space_Additions/Blueprints/BP_MIS_FirstPersonCharacter.BP_MIS_FirstPersonCharacter_C|GetDid%20Interact _refcharacter))
    (Transformation|SetActorScale3D "3.000000,3.000000,3.000000")))

(fn ConstructionScript)